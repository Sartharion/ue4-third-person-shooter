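; Base projectile Blueprint for the SciFiWeapLight weapons that handles impact effects.
; On impact it spawns a metal impact particle at its location, with pitch flipped 180 degrees to face back along its rotation.
; A Pawn cast on the hit actor selects between body and surface impact sounds, while the particle is the same for both.
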(event `self.OnImpact`
  (params (OtherActor :type "Actor Object Reference") (OtherComp :type "PrimitiveComponent Object Reference") (NormalImpulse :type "Object.Vector Structure") (Hit :type "EngineTypes.HitResult Structure (by ref)"))
  (bind _returnvalue (`self.K2_GetActorLocation`))
  (`GameplayStatics.SpawnEmitterAtLocation` (`self.MetalImpactParticleSystem`) (`self.K2_GetActorLocation`) (`KismetMathLibrary.MakeRot` (+ (.pitch (`self.K2_GetActorRotation`)) 180.0) (.yaw (`self.K2_GetActorRotation`)) (.roll (`self.K2_GetActorRotation`))))
  (cast `Pawn` OtherActor
    (:`then`
      (`GameplayStatics.PlaySoundAtLocation` (`self.BodyImpactSound`) _returnvalue))
    (:`CastFailed`
      (`GameplayStatics.PlaySoundAtLocation` (`self.SurfaceImpactSound`) _returnvalue))))

(fn `UserConstructionScript`)